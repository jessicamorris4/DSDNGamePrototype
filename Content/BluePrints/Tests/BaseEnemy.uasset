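; BaseEnemy is a test enemy character that chases the player in a top-down game, issuing AIMoveTo every Tick while not stunned.
; Capsule hits on the player call PlayerKnockBack, then halt the enemy for a short cooldown.
; Its knockback event stuns it, decrements Health, then destroys it if Health is at or below the player's Str, otherwise launches it along the player's forward vector.
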(event OnComponentHit(CapsuleComponent)
  (params (HitComponent :type Primitive%20Component%20Object%20Reference) (OtherActor :type Actor%20Object%20Reference) (OtherComp :type Primitive%20Component%20Object%20Reference) (NormalImpulse :type Vector :default "0, 0, 0") (Hit :type Hit%20Result%20Structure%20%28by%20ref%29))
  (bind _astop_downharacter (Utilities|Casting|CastToTopDownharacter OtherActor))
  (Default|PlayerKnockBack _astop_downharacter (Transformation|GetActorForwardVector))
  (CallFunction|CoolDown))

(event Custom|knockback
  (CallFunction|Stunned)
  (bind _astop_downharacter (Utilities|Casting|CastToTopDownharacter (Game|Player|GetPlayerPawn 0)))
  (Variables|Default|SetHealth (- (Variables|Default|GetHealth) 1))
  (if (<= (Variables|Default|GetHealth) (Variables|/Game/BluePrints/TopDownharacter.TopDownharacter_C|GetStr _astop_downharacter))
    (Actor|DestroyActor)
    (else
      (Character|LaunchCharacter (* (Variables|/Game/BluePrints/TopDownharacter.TopDownharacter_C|GetForwardVector _astop_downharacter) "1000.000000,1000.000000,1000.000000") false false))))

(event Custom|Stunned
  (Variables|Default|Setenemystunned true)
  (Components|Movement|StopMovementImmediately (Variables|Character|GetCharacterMovement))
  (Utilities|FlowControl|Delay 2.0)
  (Variables|Default|Setenemystunned false))

(event Custom|CoolDown
  (Variables|Default|Setenemystunned true)
  (Components|Movement|StopMovementImmediately (Variables|Character|GetCharacterMovement))
  (Utilities|FlowControl|Delay 1.0)
  (Variables|Default|Setenemystunned false))

(event EventBeginPlay)

(event Collision|EventActorBeginOverlap
  (params (OtherActor :type Actor%20Object%20Reference)))

(event EventTick
  (params (DeltaSeconds :type Float%20%28single-precision%29))
  (if (Variables|Default|Getenemystunned)
    (Development|PrintString "enemy stunned false")
    (else
      (AI|AIMoveTo self "0, 0, 0" (Game|Player|GetPlayerPawn 0) 5.0 false))))

(fn ConstructionScript)